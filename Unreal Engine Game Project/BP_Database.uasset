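; BP_Database is an actor Blueprint that manages the title and loading screen widgets, despite its database name.
; Custom events create a hidden title widget, toggle it, or remove all widgets and show the loading screen.
; ToggleWidget flips any passed widget's visibility and, given a valid player controller and character, switches character input, mouse cursor and game pause.
; A single shared WidgetIsOn flag drives both the toggle and pause state.
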(event `Loading`
  (`self.GoToLoadingScreen`))

(event `CreatetittleWG`
  (bind _returnvalue (`|CreateWidget` "/Game/WG_tittle0.WG_tittle0_C"))
  (`UserWidget.AddToViewport` _returnvalue 0)
  (`Widget.SetVisibility` _returnvalue "Hidden"))

(event `toggleTittleWG`
  (`self.ToggleWidget` (stale `CreatetittleWG` _returnvalue)))

(fn `GoToLoadingScreen`
  (`WidgetLayoutLibrary.RemoveAllWidgets`)
  (bind _returnvalue (`|CreateWidget` "/Game/WG_Loading.WG_Loading_C"))
  (`UserWidget.AddToViewport` _returnvalue 0))

(fn `toggle pause`
  (if (`self.WidgetIsOn`)
    (`GameplayStatics.SetGamePaused` false)
    (else
      (`GameplayStatics.SetGamePaused` true))))

(fn `ToggleWidget`
  (params (widget :type "UserWidget Object Reference"))
  (bind _returnvalue (`GameplayStatics.GetPlayerController` 0))
  (bind _returnvalue_2 (`GameplayStatics.GetPlayerCharacter` 0))
  (if (`self.WidgetIsOn`)
    (`Widget.SetVisibility` widget "Hidden")
    (`/Engine/EditorBlueprintResources/StandardMacros.IsValid` _returnvalue
      (:`Is Valid`
        (`/Engine/EditorBlueprintResources/StandardMacros.IsValid` _returnvalue_2
          (:`Is Valid`
            (`self.EnableInput` _returnvalue_2 _returnvalue)
            (set `PlayerController.bShowMouseCursor` false _returnvalue)
            (`self.toggle pause`)
            (set `self.WidgetIsOn` false)))))
    (else
      (`Widget.SetVisibility` widget "Visible")
      (`/Engine/EditorBlueprintResources/StandardMacros.IsValid` _returnvalue
        (:`Is Valid`
          (`/Engine/EditorBlueprintResources/StandardMacros.IsValid` _returnvalue_2
            (:`Is Valid`
              (`self.DisableInput` _returnvalue_2 _returnvalue)
              (set `PlayerController.bShowMouseCursor` true _returnvalue)
              (`self.toggle pause`)
              (set `self.WidgetIsOn` true))))))))

(fn `UserConstructionScript`)